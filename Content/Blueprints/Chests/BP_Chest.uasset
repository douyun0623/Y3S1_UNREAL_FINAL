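; BP_Chest is an interactable treasure chest that spawns one random item the first time it is opened.
; Interact checks IsOpen, then spawns a class picked from ItemClasses above the chest, disables mesh collision and swaps to the Treasure_chest mesh.
; The random index range includes the array length, so it can land out of bounds.
; Later interactions only print an already-open message.
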(event `/Game/Blueprints/Interfaces/BPI_Interact.Interact`
  (params (Player :type "Character Object Reference"))
  (bind _staticmesh (`self.StaticMesh`))
  (if (not (`self.isOpen?`))
    (`KismetSystemLibrary.PrintString` "open")
    (set `self.isOpen?` true)
    (`|SpawnActorFromClass` (`|GetArrayItem` (`self.itemClasses`) (`KismetMathLibrary.RandomIntegerInRange` 0 (`KismetArrayLibrary.Array_Length` (`self.itemClasses`)))) (`KismetMathLibrary.MakeTransform` (+ (`self.K2_GetActorLocation`) (0.0 0.0 100.0))) "Undefined" "MultiplyWithRoot" null null)
    (`PrimitiveComponent.SetCollisionEnabled` _staticmesh "NoCollision")
    (`StaticMeshComponent.SetStaticMesh` _staticmesh "/Game/Fab/Treasure_Chest/treasure_chest.treasure_chest")
    (else
      (`KismetSystemLibrary.PrintString` "이미 열림"))))

(fn `UserConstructionScript`)