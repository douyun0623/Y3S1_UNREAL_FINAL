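; BP_Item_Dumbbell is a dumbbell item that permanently adds a flat 10 to the player's attack power when picked up.
; Its ApplyEffect event casts the passed player reference to BP_Player and increases AttackPower directly, with no removal or cap.
; Debug prints announce the pickup and show the new value.
; The file has no overlap or trigger logic of its own, as its other event nodes are disabled.
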(event `/Game/Blueprints/Interfaces/BPI_ItemEffect.ApplyEffect`
  (params (PlayerRef :type "Character Object Reference"))
  ; 아이템 획득 효과
  (`KismetSystemLibrary.PrintString` "덤벨획득공격력10추가")
  (bind _asbp_player (cast `/Game/Blueprints/Characters/BP_Player` PlayerRef))
  (bind _output_get (set `/Game/Blueprints/Characters/BP_Player.attackPower` (+ (`/Game/Blueprints/Characters/BP_Player.attackPower` _asbp_player) 10.0) _asbp_player))
  (`KismetSystemLibrary.PrintString` (`KismetStringLibrary.Conv_DoubleToString` _output_get)))

(fn `UserConstructionScript`
  (`parent.UserConstructionScript`))