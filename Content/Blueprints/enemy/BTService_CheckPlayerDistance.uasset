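; Behavior tree service that updates whether an enemy is close enough to attack the player.
; Each AI tick, it reads the player from the blackboard, cast to BP_Player, and measures its straight-line distance to the controlled pawn.
; It sets the CanAttack blackboard bool true within a fixed radius and false beyond it, leaving it untouched when the cast fails.
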(event `self.ReceiveTickAI`
  (params (OwnerController :type "AIController Object Reference") (ControlledPawn :type "Pawn Object Reference") (DeltaSeconds :type "Float (single-precision)"))
  (bind _canattack (`self.CanAttack`))
  (bind _asbp_player (cast `/Game/Blueprints/Characters/BP_Player` (`BTFunctionLibrary.GetBlackboardValueAsObject` (`self.playerKey`))))
  (if (<= (`KismetMathLibrary.VSize` (- (`Actor.K2_GetActorLocation` _asbp_player) (`Actor.K2_GetActorLocation` ControlledPawn))) 400.0)
    (`BTFunctionLibrary.SetBlackboardValueAsBool` _canattack true)
    (else
      (`BTFunctionLibrary.SetBlackboardValueAsBool` _canattack))))