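; BP_BreakableObject is a breakable mineral actor that drops a coin when destroyed.
; Point damage is subtracted from its HP, with debug prints of the prior HP and a hit message.
; Once HP falls below zero, it destroys itself and spawns a BP_Coin at its location.
; The AnyDamage, overlap, tick and BeginPlay events are empty.
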(event `self.ReceiveAnyDamage`
  (params (Damage :type "Float (single-precision)") (DamageType :type "DamageType Object Reference") (InstigatedBy :type "Controller Object Reference") (DamageCauser :type "Actor Object Reference")))

(event `self.ReceivePointDamage`
  (params (Damage :type "Float (single-precision)") (DamageType :type "DamageType Object Reference") (HitLocation :type "Vector Structure") (HitNormal :type "Vector Structure") (HitComponent :type "PrimitiveComponent Object Reference") (BoneName :type Name) (ShotFromDirection :type "Vector Structure") (InstigatedBy :type "Controller Object Reference") (DamageCauser :type "Actor Object Reference") (HitInfo :type "HitResult Structure (by ref)"))
  (`KismetSystemLibrary.PrintString` (`KismetStringLibrary.Conv_DoubleToString` (`self.HP`)))
  (`KismetSystemLibrary.PrintString` "광물에 데미지 ")
  (bind _output_get (set `self.HP` (- (`self.HP`) Damage)))
  (if (< _output_get 0.0)
    (`self.K2_DestroyActor`)
    (`|SpawnActorFromClass` "/Game/Blueprints/Items/BP_Coin.BP_Coin_C" (`KismetMathLibrary.Conv_VectorToTransform` (`self.K2_GetActorLocation`)) "AlwaysSpawn" "MultiplyWithRoot" null (struct) null)))

(fn `UserConstructionScript`)