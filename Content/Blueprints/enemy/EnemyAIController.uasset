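; AI controller for enemy pawns that runs the Enemy_BT behavior tree and tells it which player to target.
; On possess it starts the tree and copies the pawn's AttackMontage from BP_Enemy into the Blackboard.
; AI perception updates set TargetPlayer when an actor tagged PLAYER is sensed and clear it when that actor is lost.
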(event `self.ReceivePossess`
  (params (PossessedPawn :type "Pawn Object Reference"))
  (`self.RunBehaviorTree` "/Game/Blueprints/enemy/Enemy_BT.Enemy_BT")
  (bind _asbp_enemy (cast `/Game/Blueprints/enemy/BP_Enemy` PossessedPawn))
  (`BlackboardComponent.SetValueAsObject` (`self.Blackboard`) "AttackMontage" (`/Game/Blueprints/enemy/BP_Enemy.AttackMontage` _asbp_enemy)))

(event `self.AIPerception.OnTargetPerceptionUpdated`
  (params (Actor :type "Actor Object Reference") (Stimulus :type "AIStimulus Structure"))
  (bind _blackboard (`self.Blackboard`))
  (if (`self.ActorHasTag` Actor "PLAYER")
    (if Stimulus_bSuccessfullySensed
      (`BlackboardComponent.SetValueAsObject` _blackboard "TargetPlayer" Actor)
      (else
        (`BlackboardComponent.ClearValue` _blackboard "TargetPlayer")))))

(fn `UserConstructionScript`)