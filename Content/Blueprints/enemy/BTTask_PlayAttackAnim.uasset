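; Behavior tree task that plays an enemy's attack montage and applies melee damage to the player.
; It plays the blackboard-supplied montage from its Attack section on the BP_Enemy mesh.
; The AttackHitCheck notify triggers a debug-drawn sphere trace at the HitPoint socket, using the enemy's Range and Damage to hurt a hit BP_Player.
; Only montage completion clears a blackboard bool and finishes the task; interruption and failed casts never finish it.
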(event `self.ReceiveExecuteAI`
  (params (OwnerController :type "AIController Object Reference") (ControlledPawn :type "Pawn Object Reference"))
  (bind _asbp_enemy (cast `/Game/Blueprints/enemy/BP_Enemy` ControlledPawn))
  (bind _asanim_montage (cast `AnimMontage` (`BTFunctionLibrary.GetBlackboardValueAsObject` (`self.MontageKey`))))
  (bind _notifyname (`|PlayMontage` (`Character.Mesh` _asbp_enemy) _asanim_montage 1.0 0.0 "Attack")
    (:`OnCompleted`
      (`BTFunctionLibrary.SetBlackboardValueAsBool` (`self.Key`))
      (`self.FinishExecute` true))
    (:`OnNotifyBegin`
      (if (== _notifyname "AttackHitCheck")
        (bind _returnvalue (`SceneComponent.GetSocketLocation` (`Character.Mesh` _asbp_enemy) "HitPoint"))
        (bind _outhit (`KismetSystemLibrary.SphereTraceSingle` :`Start` _returnvalue :`End` _returnvalue :`Radius` (`/Game/Blueprints/enemy/BP_Enemy.Range` _asbp_enemy) :`TraceChannel` "TraceTypeQuery1" :`DrawDebugType` "Persistent"))
        (bind _asbp_player (cast `/Game/Blueprints/Characters/BP_Player` (`.HitActor` (`GameplayStatics.BreakHitResult` _outhit))))
        (`KismetSystemLibrary.PrintString` "적공격성공데미지들어가나?")
        (`GameplayStatics.ApplyDamage` _asbp_player (`/Game/Blueprints/enemy/BP_Enemy.Damage` _asbp_enemy))))))