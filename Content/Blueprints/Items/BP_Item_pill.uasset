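; BP_Item_pill is a pill item that boosts the player's health when its effect is applied.
; ApplyEffect casts the passed player reference to BP_Player, then adds the same fixed amount to both HP and MaxHP.
; It prints a Korean pickup message and the new MaxHP, while BeginPlay, overlap and Tick are unused stubs in this file.
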(event `/Game/Blueprints/Interfaces/BPI_ItemEffect.ApplyEffect`
  (params (PlayerRef :type "Character Object Reference"))
  (`KismetSystemLibrary.PrintString` "알약1획득체력10추가")
  (bind _asbp_player (cast `/Game/Blueprints/Characters/BP_Player` PlayerRef))
  (set `/Game/Blueprints/Characters/BP_Player.HP` (+ (`/Game/Blueprints/Characters/BP_Player.HP` _asbp_player) 10.0) _asbp_player)
  (bind _output_get (set `/Game/Blueprints/Characters/BP_Player.MaxHP` (+ (`/Game/Blueprints/Characters/BP_Player.MaxHP` _asbp_player) 10.0) _asbp_player))
  (`KismetSystemLibrary.PrintString` (`KismetStringLibrary.Conv_DoubleToString` _output_get)))

(fn `UserConstructionScript`
  (`parent.UserConstructionScript`))