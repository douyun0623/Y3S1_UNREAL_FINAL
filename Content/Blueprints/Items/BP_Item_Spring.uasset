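; BP_Item_Spring is an item that permanently grants the player one extra jump, then removes itself.
; Its ApplyEffect event casts the passed PlayerRef to BP_Player, increments MaxJump and destroys the item actor.
; Debug prints report the effect and the new jump count.
; The file holds no overlap or trigger logic, so ApplyEffect relies on being invoked from outside this graph.
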(event `/Game/Blueprints/Interfaces/BPI_ItemEffect.ApplyEffect`
  (params (PlayerRef :type "Character Object Reference"))
  (`KismetSystemLibrary.PrintString` "점프추가")
  (bind _asbp_player (cast `/Game/Blueprints/Characters/BP_Player` PlayerRef))
  (bind _output_get (set `/Game/Blueprints/Characters/BP_Player.MaxJump` (+ (`/Game/Blueprints/Characters/BP_Player.MaxJump` _asbp_player) 1) _asbp_player))
  (`KismetSystemLibrary.PrintString` (`KismetStringLibrary.Conv_IntToString` _output_get))
  (`self.K2_DestroyActor`))

(fn `UserConstructionScript`
  (`parent.UserConstructionScript`))