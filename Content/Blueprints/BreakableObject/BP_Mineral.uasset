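; BP_Mineral is a mineral prop in the BreakableObject set that varies its look per instance and reacts to hits.
; Its construction script picks one of four materials, a random per-axis mesh scale and a random yaw.
; On point damage it calls the parent handler, then spawns an explosion particle at the hit location.
; It adds no breaking logic of its own.
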(event `self.ReceivePointDamage`
  (params (Damage :type "Float (single-precision)") (DamageType :type "DamageType Object Reference") (HitLocation :type "Vector Structure") (HitNormal :type "Vector Structure") (HitComponent :type "PrimitiveComponent Object Reference") (BoneName :type Name) (ShotFromDirection :type "Vector Structure") (InstigatedBy :type "Controller Object Reference") (DamageCauser :type "Actor Object Reference") (HitInfo :type "HitResult Structure (by ref)"))
  (`parent.ReceivePointDamage` Damage null HitLocation (0.0 0.0 0.0) null "None" (0.0 0.0 0.0) null null HitInfo)
  (`GameplayStatics.SpawnEmitterAtLocation` "/Game/StarterContent/Particles/P_Explosion.P_Explosion" HitLocation))

(fn `UserConstructionScript`
  (bind _returnvalue (`KismetMathLibrary.RandomFloatInRange` 1.0 3.0))
  (`parent.UserConstructionScript`)
  (`PrimitiveComponent.SetMaterial` (`self.StaticMesh`) 0 (`|GetArrayItem` (`self.MaterialList`) (`KismetMathLibrary.RandomIntegerInRange` 0 3)))
  (`SceneComponent.SetWorldScale3D` (`self.StaticMesh`) (`KismetMathLibrary.MakeVector` _returnvalue _returnvalue _returnvalue))
  (`self.K2_SetActorRotation` (`KismetMathLibrary.MakeRotator` 0.0 0.0 (`KismetMathLibrary.RandomFloatInRange` 0.0 360.0))))